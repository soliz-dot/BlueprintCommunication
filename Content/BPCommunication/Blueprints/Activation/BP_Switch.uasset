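; BP_Switch is a trigger switch that turns on when a BP_Cube enters it and moves the referenced Roca actor to a hardcoded location.
; Activation swaps the Switch mesh to OnMaterial, while the construction script starts it on OffMaterial.
; Unless ActivateOnce is set, emptying the trigger of all actors restores OffMaterial and prints a hint to find the cube, leaving Roca in place.
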(event OnComponentBeginOverlap(Trigger)
  (params (OverlappedComponent :type Primitive%20Component%20Object%20Reference) (OtherActor :type Actor%20Object%20Reference) (OtherComp :type Primitive%20Component%20Object%20Reference) (OtherBodyIndex :type Integer) (bFromSweep :type Boolean) (SweepResult :type Hit%20Result%20Structure%20%28by%20ref%29))
  (Utilities|Casting|CastToBP_Cube OtherActor)
  (Rendering|Material|SetMaterial (Variables|Default|GetSwitch) 0 (Variables|Setup|GetOnMaterial))
  (Transformation|SetActorLocation (Variables|Default|GetRoca) "5521.000000,-1882.949020,392.000000" false false))

(event OnComponentEndOverlap(Trigger)
  (params (OverlappedComponent :type Primitive%20Component%20Object%20Reference) (OtherActor :type Actor%20Object%20Reference) (OtherComp :type Primitive%20Component%20Object%20Reference) (OtherBodyIndex :type Integer))
  (if (not (Variables|Setup|GetActivateOnce))
    (if (Utilities|Array|IsEmpty (Collision|GetOverlappingActors (Variables|Default|GetTrigger) "/Script/Engine.Actor" :!class /Script/Engine.PrimitiveComponent))
      (Rendering|Material|SetMaterial (Variables|Default|GetSwitch) 0 (Variables|Setup|GetOffMaterial))
      (Development|PrintString "Look for the cube"))))

(fn ConstructionScript
  (Rendering|Material|SetMaterial (Variables|Default|GetSwitch) 0 (Variables|Setup|GetOffMaterial)))